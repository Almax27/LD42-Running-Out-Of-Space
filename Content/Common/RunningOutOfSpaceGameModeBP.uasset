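; Game mode for Running Out Of Space: plays music, counts kills, saves the high score and reloads the level after player death.
; Player spawn starts a self-re-arming timer whose interval inverts a randomly jittered spawn-rate curve over elapsed time.
; Each tick calls NavSpawn, but its spider-spawning logic at random reachable points near the player is disconnected, so nothing spawns.
; Kills are broadcast with the running total.
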(event `self.ReceiveBeginPlay`
  (`|ExecutionSequence`
    (:`then_0`
      (bind _returnvalue (`GameplayStatics.LoadGameFromSlot` "SaveGame"))
      (bind _asrunning_out_of_space_save_game (cast `/Game/Common/RunningOutOfSpaceSaveGame` _returnvalue)
        (:`then`
          (set `self.SaveGame` _asrunning_out_of_space_save_game))
        (:`CastFailed`
          (bind _returnvalue_2 (`GameplayStatics.CreateSaveGameObject` "/Game/Common/RunningOutOfSpaceSaveGame.RunningOutOfSpaceSaveGame_C"))
          (set `self.SaveGame` _returnvalue_2))))
    (:`then_1`
      (`GameplayStatics.PlaySound2D` "/Game/Audio/bensound-deepblue.bensound-deepblue" 1.0 1.0 0.0 null null))))

(event `Event EnemyKilled`
  (params (EnemyKilled :type "Actor Object Reference"))
  (bind _result (`/Engine/EditorBlueprintResources/StandardMacros.IncrementInt` (`self.KillCount`))
    (:`  `
      (`self.OnEnemyKilled` EnemyKilled _result))))

(event `Event PlayerSpawn`
  (set `self.GameStartTime` (`GameplayStatics.GetTimeSeconds`))
  (`KismetSystemLibrary.K2_SetTimerDelegate` (delegate `TestSpawn`) (`self.GetSpawnRate`) :!label _label)
  (`self.NavSpawn`))

(event `TestSpawn`
  (`self.NavSpawn`)
  (goto _label))

(event `Event PlayerDeath`
  (bind _savegame (`self.SaveGame`))
  (bind _returnvalue (* (`self.KillCount`) 100))
  (if (> _returnvalue (`/Game/Common/RunningOutOfSpaceSaveGame.HighScore` _savegame))
    (set `/Game/Common/RunningOutOfSpaceSaveGame.HighScore` _returnvalue _savegame))
  (`GameplayStatics.SaveGameToSlot` _savegame "SaveGame")
  (`KismetSystemLibrary.Delay` 3.0)
  (bind _returnvalue_2 (`GameplayStatics.GetCurrentLevelName` true))
  (`GameplayStatics.OpenLevel` (`KismetStringLibrary.Conv_StringToName` _returnvalue_2)))

(fn `GetSpawnRate`
  (returns (SpawnRate :type "Float (double-precision)"))
  (bind _returnvalue (* (`CurveFloat.GetFloatValue` (`self.SpawnRateCurve`) (- (`GameplayStatics.GetTimeSeconds`) (`self.GameStartTime`))) (`KismetMathLibrary.RandomFloatInRange` 0.9 1.1)))
  (if (> _returnvalue 0.0)
    (return (/ 1.0 _returnvalue))
    (else
      (return 0.0))))

(fn `NavSpawn`
  (returns (Spawned :type "Character Object Reference")))

(fn `UserConstructionScript`)