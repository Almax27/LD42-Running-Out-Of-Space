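; Player soul Blueprint that drives the look of its SoulTrail particle trail as the soul changes state.
; It extends the parent's state-entry handling, starting a white trail when following, turning it red on a critical throw and ending it when returning.
; The tint is applied through the trail's color parameter, which is also set to white at BeginPlay.
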(event `self.ReceiveBeginPlay`
  (`ParticleSystemComponent.SetColorParameter` (`self.SoulTrail`) "TrailColor" (struct :`R` 1.0 :`G` 1.0 :`B` 1.0 :`A` 1.0)))

(event `self.OnEnterState`
  (params (NewState :type "EPlayerSoulState Enum" :default "None"))
  (bind _soultrail (`self.SoulTrail`))
  (`parent.OnEnterState` NewState)
  (switch `EPlayerSoulState` NewState
    (:`Following`
      (`|ExecutionSequence`
        (:`then_0`
          (`ParticleSystemComponent.SetColorParameter` _soultrail "TrailColor" (struct :`R` 1.0 :`G` 1.0 :`B` 1.0 :`A` 1.0))
          (`ParticleSystemComponent.BeginTrails` _soultrail "None" "None" "ETrailWidthMode_FromCentre" 10.0))))
    (:`ThrownCritical`
      (`ParticleSystemComponent.SetColorParameter` _soultrail "TrailColor" (struct :`R` 1.0 :`A` 1.0)))
    (:`Returning`
      (`ParticleSystemComponent.EndTrails` _soultrail))))

(fn `UserConstructionScript`)